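; Actor component that tracks health for its owner, initialized to MaxHealth on BeginPlay.
; Damage and Heal ignore negative amounts and clamp Health between zero and MaxHealth, alongside dead-state and normalized-health getters.
; Tick regenerates health only when the owner is player character 0, chaining a fixed Delay, a debug print and a rate Delay before healing.
; The fixed delay runs independently of when damage occurs.
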(event EventBeginPlay
  (CallFunction|Init (Variables|Setup|GetMaxHealth)))

(event EventTick
  (params (DeltaSeconds :type Float%20%28single-precision%29))
  ;[1 1 1] Health Regen for player only
  (if (== (Game|GetPlayerCharacter 0) (Components|GetOwner))
    (if (< (CallFunction|GetHealth) (Variables|Setup|GetMaxHealth))
      (Utilities|FlowControl|Delay 15.0)
      (Development|PrintString (Utilities|String|ToString(Float) (CallFunction|GetHealth)))
      (Utilities|FlowControl|Delay (Variables|Setup|GetHealthRegenRate))
      (CallFunction|Heal (Variables|Setup|GetHealthRegenAmount)))))

(fn Init
  (params (MaxHealth :type Float%20%28double-precision%29))
  (Variables|Setup|SetHealth MaxHealth))

(fn Damage
  (params (Amount :type Float%20%28double-precision%29))
  (if (not (< Amount 0.0))
    (Utilities|ClampSetHealth (- (Variables|Setup|GetHealth) Amount))))

(fn Heal
  (params (Amount :type Float%20%28double-precision%29))
  (if (not (< Amount 0.0))
    (Utilities|ClampSetHealth (+ (Variables|Setup|GetHealth) Amount))))

(fn IsDead
  (return (<= (Variables|Setup|GetHealth) 0.0)))

(fn GetHealth
  (return (Variables|Setup|GetHealth)))

(fn GetNormalizedHealth
  (return (Math|Float|Clamp(Float) (/ (Variables|Setup|GetHealth) (Variables|Setup|GetMaxHealth)))))