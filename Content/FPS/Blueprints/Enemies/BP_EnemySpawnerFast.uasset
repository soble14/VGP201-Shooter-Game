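; Enemy spawner actor that periodically adds BP_AICharacterFast enemies to the level until a maximum count is reached.
; A looping timer started on BeginPlay calls SpawnEnemy, which takes X and Y from random reachable navmesh points in a very large radius around the spawner, with a fixed Z.
; The counter only increments here, so MaxEnemies limits total spawns unless something external lowers it.
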(event Custom|Spawn%20Enemy
  (bind _returnvalue (Transformation|GetActorLocation))
  (bind _randomlocation (AI|Navigation|GetRandomReachablePointinRadius _returnvalue 1e+05 0 0))
  (if (< (Variables|Default|GetCurrentEnemyCount) (Variables|Default|GetMaxEnemies))
    (Development|PrintString "Spawning Enemy")
    (Game|SpawnActorfromClass "/Game/FPS/Blueprints/Enemies/EnemyAI/BP_AICharacterFast.BP_AICharacterFast_C" (Math|Transform|MakeTransform (Math|Vector|MakeVector (.x _randomlocation) (.y _randomlocation) 2e+02) "0, 0, 0" "1.000000,1.000000,1.000000") "Undefined" "MultiplyWithRoot" 0 0)
    (bind _result (Math|Integer|IncrementInt (Variables|Default|GetCurrentEnemyCount))
      (:%20%20
        (Variables|Default|SetCurrentEnemyCount _result)))
    (else
      (Development|PrintString "Max Enemies Spawned"))))

(event EventBeginPlay
  (Utilities|Time|SetTimerbyEvent (delegate Custom|Spawn%20Enemy) 1e+01 true))

(fn ConstructionScript)