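; BP_AICharacterBoss is a boss enemy in the FPS game that takes damage and drops coins on death.
; AnyDamage routes into TakeDamage, which applies the amount to a Health component and checks whether it is dead.
; On death it spawns ten BP_Coin actors at its location and destroys itself; otherwise it prints remaining health.
; No AI behavior is defined in these graphs.
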(event Game|Damage|EventAnyDamage
  (params (Damage :type Float%20%28single-precision%29) (DamageType :type Damage%20Type%20Object%20Reference) (InstigatedBy :type Controller%20Object%20Reference) (DamageCauser :type Actor%20Object%20Reference))
  (CallFunction|TakeDamage Damage))

(event EventBeginPlay
  (Development|PrintString "Enemy Initialized"))

(fn ConstructionScript)

(fn TakeDamage
  (params (Damage :type Float%20%28double-precision%29))
  (bind _health (Variables|Default|GetHealth))
  (Default|Damage _health Damage)
  (if (Default|IsDead _health)
    (for _index (range 0 9)
      (Game|SpawnActorfromClass "/Game/FPS/Blueprints/Collectables/BP_Coin.BP_Coin_C" (Math|Transform|MakeTransform (Transformation|GetActorLocation) "0, 0, 0" "1.000000,1.000000,1.000000") "Undefined" "MultiplyWithRoot" 0 0))
    (Actor|DestroyActor)
    (else
      (Development|PrintString (Utilities|String|ToString(Float) (Default|GetHealth _health))))))