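; GM_FPSGameMode is the game mode for an FPS game that owns the HUD and the player's score.
; On BeginPlay it creates the reticle and game UI widgets, adds both to the viewport, and initializes the health bar to full and the score display.
; AddScore adds points to the score and pushes the new total to the game UI widget.
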(event EventBeginPlay
  (Development|PrintString "Spawing FPSGameMode" true true "(R=0.843750,G=0.000000,B=0.152070,A=1.000000)")
  (bind _returnvalue (UserInterface|CreateWidget "/Game/FPS/Blueprints/UI/WBP_Reticle.WBP_Reticle_C"))
  (UserInterface|Viewport|AddtoViewport _returnvalue 0)
  (bind _returnvalue_2 (UserInterface|CreateWidget "/Game/FPS/Blueprints/UI/WBP_GameUI.WBP_GameUI_C"))
  (bind _output_get (Variables|Default|SetGame%20UI _returnvalue_2))
  (UserInterface|Viewport|AddtoViewport _output_get 0)
  (Default|SetHealthBar (Variables|Default|GetGame%20UI) 1.0)
  (Default|SetScore (Variables|Default|GetGame%20UI) (Variables|Default|GetScore)))

(event EventTick
  (params (DeltaSeconds :type Float%20%28single-precision%29)))

(fn ConstructionScript)

(fn AddScore
  (params (Points :type Integer))
  (bind _output_get (Variables|Default|SetScore (+ (Variables|Default|GetScore) Points)))
  (Default|SetScore (Variables|Default|GetGame%20UI) _output_get))